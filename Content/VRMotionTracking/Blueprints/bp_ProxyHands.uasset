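; Proxy hands actor that mirrors the VR pawn's Oculus hand tracking onto left and right poseable hand meshes.
; UpdateProxyHands copies live pawn transforms into per-joint components when IsLive, then always poses bones from them in component space, gated by StartHandMirrorTick.
; BeginPlay only fills proxy component arrays, which go unused here.
; Setup of that gate, meshes, bone names and tagged transform arrays sits in disconnected nodes.
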(event `self.ReceiveTick`
  (params (DeltaSeconds :type "Float (single-precision)")))

(event `self.ReceiveBeginPlay`
  (`|ExecutionSequence`
    (:`then_0`
      (set `self.rh_proxyArray` (`|MakeArray` (`self.transform4`) (`self.transform5`) (`self.transform6`) (`self.transform7`) (`self.transform8`) (`self.transform9`) (`self.transform10`) (`self.transform11`) (`self.transform12`) (`self.transform13`) (`self.transform14`) (`self.transform15`) (`self.transform16`) (`self.transform17`) (`self.transform18`) (`self.transform19`) (`self.transform21`) (`self.transform22`) (`self.transform23`) (`self.transform24`)))
      (set `self.lh_proxyArray` (`|MakeArray` (`self.transform28`) (`self.transform29`) (`self.transform30`) (`self.transform31`) (`self.transform32`) (`self.transform33`) (`self.transform34`) (`self.transform35`) (`self.transform36`) (`self.transform37`) (`self.transform38`) (`self.transform39`) (`self.transform40`) (`self.transform41`) (`self.transform42`) (`self.transform43`) (`self.transform45`) (`self.transform46`) (`self.transform47`) (`self.transform48`))))))

(event `UpdateProxyHands`
  (if (`self.StartHandMirrorTick`)
    (`|ExecutionSequence`
      (:`then_0`
        (if (`self.isLive`)
          (for (_array_element _array_index) (`/Game/VRMotionTracking/Blueprints/VRPawn_lvl1.RightHandTransArray` (`self.vrpawn`))
            (`SceneComponent.K2_SetRelativeTransform` (`|GetArrayItem` (`self.rh_transformsArray`) _array_index) (`KismetMathLibrary.MakeTransform` (.location _array_element) (.rotation _array_element) (0.01 0.01 0.01)) false false))
          (for (_array_element_2 _array_index_2) (`/Game/VRMotionTracking/Blueprints/VRPawn_lvl1.LeftHandTransArray` (`self.vrpawn`))
            (`SceneComponent.K2_SetRelativeTransform` (`|GetArrayItem` (`self.lh_transformsArray`) _array_index_2) (`KismetMathLibrary.MakeTransform` (.location _array_element_2) (.rotation _array_element_2) (0.01 0.01 0.01)) false false))))
      (:`then_1`
        (for (_array_element_3 _array_index_3) (`self.Bone Array Oculus Hand`)
          (bind (_returnvalue_location _returnvalue_rotation) (`KismetMathLibrary.BreakTransform` (`SceneComponent.GetRelativeTransform` (`|GetArrayItem` (`self.rh_transformsArray`) _array_index_3))))
          (`PoseableMeshComponent.SetBoneTransformByName` (`self._ProxyHandRight`) _array_element_3 (`KismetMathLibrary.MakeTransform` (+ _returnvalue_location (0.0 0.0 0.0)) _returnvalue_rotation) "ComponentSpace")))
      (:`then_2`
        (for (_array_element_4 _array_index_4) (`self.Bone Array Oculus Hand`)
          (bind (_returnvalue_location_2 _returnvalue_rotation_2) (`KismetMathLibrary.BreakTransform` (`SceneComponent.GetRelativeTransform` (`|GetArrayItem` (`self.lh_transformsArray`) _array_index_4))))
          (`PoseableMeshComponent.SetBoneTransformByName` (`self._ProxyHandLeft`) _array_element_4 (`KismetMathLibrary.MakeTransform` (+ _returnvalue_location_2 (0.0 0.0 0.0)) _returnvalue_rotation_2) "ComponentSpace"))))))

(fn `UserConstructionScript`)