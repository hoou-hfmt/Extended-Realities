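; PC_LevelOne is the level-one player controller, handling avatar possession and switching between four camera views.
; On BeginPlay it has GM_LevelOne possess the avatar, then runs four actor lookups but sets Cam1–Cam4 to None.
; SetCam1–4 events each activate that camera's component and switch to it using an ease-in-out view-target blend.
; Possession prints a debug message, while the 3D text event is an empty stub.
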(event `self.ReceiveBeginPlay`
  (`|ExecutionSequence`
    (:`then_0`
      (bind _asgm_level_one (cast `/Game/VRMotionTracking/Blueprints/GM_LevelOne` (`GameplayStatics.GetGameMode`)))
      (`/Game/VRMotionTracking/Blueprints/GM_LevelOne.PossessPlayerToAvatar` _asgm_level_one self))
    (:`then_1`
      (`|ExecutionSequence`
        (:`then_0`
          (bind _returnvalue (`GameplayStatics.GetActorOfClass` null))
          (set `self.Cam1` null _returnvalue))
        (:`then_1`
          (bind _returnvalue_2 (`GameplayStatics.GetActorOfClass` null))
          (set `self.Cam2` null _returnvalue_2))
        (:`then_2`
          (bind _returnvalue_3 (`GameplayStatics.GetActorOfClass` null))
          (set `self.Cam3` null _returnvalue_3))
        (:`then_3`
          (bind _returnvalue_4 (`GameplayStatics.GetActorOfClass` null))
          (set `self.Cam4` null _returnvalue_4))))))

(event `self.ReceivePossess`
  (params (PossessedPawn :type "Pawn Object Reference"))
  (`KismetSystemLibrary.PrintString` (`KismetStringLibrary.Concat_StrStr` "Controller Possessed " (`KismetSystemLibrary.GetDisplayName` PossessedPawn)) true true (struct :`R` 0.210392 :`G` 1.0 :`B` 0.890193 :`A` 1.0) 5.0))

(event `SetCam1`
  (bind (_cam1 _cam1_2) (`self.Cam1`))
  (`ActorComponent.Activate` (`/Game/VRMotionTracking/Blueprints/PC_LevelOne.Camera` _cam1_2) true)
  (`self.SetViewTargetWithBlend` _cam1_2 0.0 "VTBlend_EaseInOut"))

(event `SetCam2`
  (bind (_cam2 _cam2_2) (`self.Cam2`))
  (`ActorComponent.Activate` (`/Game/VRMotionTracking/Blueprints/PC_LevelOne.Camera` _cam2_2) true)
  (`self.SetViewTargetWithBlend` _cam2_2 0.0 "VTBlend_EaseInOut"))

(event `SetCam3`
  (bind (_cam3 _cam3_2) (`self.Cam3`))
  (`ActorComponent.Activate` (`/Game/VRMotionTracking/Blueprints/PC_LevelOne.Camera` _cam3_2) true)
  (`self.SetViewTargetWithBlend` _cam3_2 0.0 "VTBlend_EaseInOut"))

(event `SetCam4`
  (bind (_cam4 _cam4_2) (`self.Cam4`))
  (`ActorComponent.Activate` (`/Game/VRMotionTracking/Blueprints/PC_LevelOne.Camera` _cam4_2) true)
  (`self.SetViewTargetWithBlend` _cam4_2 0.0 "VTBlend_EaseInOut"))

(event `/3dtext/text`
  (params (`3dText` :type Text)))

(fn `UserConstructionScript`)