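; OSC control actor that drives the VR pawn's score text and the 3D text on cameras from address-named message events.
; BeginPlay caches VRPawn_lvl1 and, after a short delay, finds Bp_CAMERAS but sets CamArray to None, leaving that actor's array unconnected.
; Score messages update the pawn.
; 3D text messages loop over CamArray, setting text, size or per-axis relative position, with floats range-mapped and clamped.
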(event `self.ReceiveBeginPlay`
  (`|ExecutionSequence`
    (:`then_0`
      (bind _returnvalue (`GameplayStatics.GetActorOfClass` "/Game/VRMotionTracking/Blueprints/VRPawn_lvl1.VRPawn_lvl1_C"))
      (set `self.VRPawn` _returnvalue))
    (:`then_1`
      (`KismetSystemLibrary.Delay` 0.2)
      (bind _returnvalue_2 (`GameplayStatics.GetActorOfClass` "/Game/VRMotionTracking/Blueprints/OSCControl/bp_CAMERAS.bp_CAMERAS_C"))
      (set `self.Cam Array` _ (`.CamArray` (`/Game/VRMotionTracking/Blueprints/OSCControl/bp_CAMERAS.CamArray` _returnvalue_2))))))

(event `/score/text`
  (params (Message :type "OSCMessage Structure"))
  (bind _value (`OSCManager.GetString` Message))
  (bind _output_get (set `self.ScoreText_Performer` (`KismetTextLibrary.Conv_StringToText` _value)))
  (`/Game/VRMotionTracking/Blueprints/VRPawn_lvl1.SetScoreText` (`self.VRPawn`) _output_get))

(event `/3dtext/text`
  (params (Message :type "OSCMessage Structure"))
  (bind _value (`OSCManager.GetString` Message))
  (bind _output_get (set `self.3DText` (`KismetTextLibrary.Conv_StringToText` _value)))
  (for _array_element (`.Cam Array` (`self.Cam Array`))
    (`TextRenderComponent.K2_SetText` (`/Game/VRMotionTracking/Blueprints/OSCControl/bp_SCORE.3DText` _array_element) _output_get)))

(event `/3dtext/fontsize`
  (params (Message :type "OSCMessage Structure"))
  (bind _value (`OSCManager.GetFloat` Message))
  (for _array_element (`.Cam Array` (`self.Cam Array`))
    (`TextRenderComponent.SetWorldSize` (`/Game/VRMotionTracking/Blueprints/OSCControl/bp_SCORE.3DText` _array_element) (`KismetMathLibrary.MapRangeClamped` _value 0.0 1.0 0.0 10.0))))

(event `/3dtext/pos/x`
  (params (Message :type "OSCMessage Structure"))
  (bind (_3dtextrelativeloc_x _3dtextrelativeloc_y _3dtextrelativeloc_z) (`KismetMathLibrary.BreakVector` (`self.3DTextRelativeLoc`)))
  (bind _value (`OSCManager.GetFloat` Message))
  (set `self.3DTextRelativeLoc` (`KismetMathLibrary.MakeVector` (`KismetMathLibrary.MapRangeClamped` _value 0.0 1.0 50.0 -50.0) _3dtextrelativeloc_y _3dtextrelativeloc_z))
  (for _array_element (`.Cam Array` (`self.Cam Array`))
    (`SceneComponent.K2_SetRelativeLocation` (`/Game/VRMotionTracking/Blueprints/OSCControl/bp_SCORE.3DText` _array_element) (`self.3DTextRelativeLoc`) false false)))

(event `/3dtext/pos/y`
  (params (Message :type "OSCMessage Structure"))
  (bind (_3dtextrelativeloc_x _3dtextrelativeloc_y _3dtextrelativeloc_z) (`KismetMathLibrary.BreakVector` (`self.3DTextRelativeLoc`)))
  (bind _value (`OSCManager.GetFloat` Message))
  (set `self.3DTextRelativeLoc` (`KismetMathLibrary.MakeVector` _3dtextrelativeloc_x (`KismetMathLibrary.MapRangeClamped` _value 0.0 1.0 50.0 -50.0) _3dtextrelativeloc_z))
  (for _array_element (`.Cam Array` (`self.Cam Array`))
    (`SceneComponent.K2_SetRelativeLocation` (`/Game/VRMotionTracking/Blueprints/OSCControl/bp_SCORE.3DText` _array_element) (`self.3DTextRelativeLoc`) false false)))

(event `/3dtext/pos/z`
  (params (Message :type "OSCMessage Structure"))
  (bind (_3dtextrelativeloc_x _3dtextrelativeloc_y) (`KismetMathLibrary.BreakVector` (`self.3DTextRelativeLoc`)))
  (bind _value (`OSCManager.GetFloat` Message))
  (set `self.3DTextRelativeLoc` (`KismetMathLibrary.MakeVector` _3dtextrelativeloc_x _3dtextrelativeloc_y (`KismetMathLibrary.MapRangeClamped` _value 0.0 1.0 20.0 -20.0)))
  (for _array_element (`.Cam Array` (`self.Cam Array`))
    (`SceneComponent.K2_SetRelativeLocation` (`/Game/VRMotionTracking/Blueprints/OSCControl/bp_SCORE.3DText` _array_element) (`self.3DTextRelativeLoc`) false false)))

(fn `UserConstructionScript`)