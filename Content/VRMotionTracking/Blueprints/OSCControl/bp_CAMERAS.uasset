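; OSC-controlled manager for the spectator cameras (free, front, top, POV) in a VR motion-tracking level.
; Camera selection feeds the chosen scene capture to the spectator screen when the HMD is active, otherwise calls the player controller.
; Position and rotation messages move the free camera through timelines with play rates derived from millisecond durations.
; Zoom sets a target FOV that Tick eases toward, and a lock-to-avatar message toggles each camera's lock.
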(event `self.ReceiveBeginPlay`
  (`|ExecutionSequence`
    (:`then_0`
      (`|ExecutionSequence`
        (:`then_0`
          (bind _returnvalue (`GameplayStatics.GetActorOfClass` "/Game/VRMotionTracking/Blueprints/VRPawn_lvl1.VRPawn_lvl1_C"))
          (set `self.VRPawn_lvl1` _returnvalue))
        (:`then_1`
          (bind _returnvalue_2 (`GameplayStatics.GetActorOfClass` null))
          (set `self.SpecCam_Free` null _returnvalue_2))
        (:`then_2`
          (bind _returnvalue_3 (`GameplayStatics.GetActorOfClass` null))
          (set `self.SpecCam_Front` null _returnvalue_3))
        (:`then_3`
          (bind _returnvalue_4 (`GameplayStatics.GetActorOfClass` null))
          (set `self.SpecCam_Top` null _returnvalue_4))
        (:`then_4`
          (bind _returnvalue_5 (`GameplayStatics.GetActorOfClass` null))
          (set `self.SpecCam_POV` null _returnvalue_5))
        (:`then_5`
          (bind _returnvalue_6 (`GameplayStatics.GetActorOfClass` null))
          (set `self.SpecCam_Main` null _returnvalue_6))))
    (:`then_1`
      (bind _returnvalue_7 (`GameplayStatics.GetActorOfClass` "/Game/VRMotionTracking/Blueprints/PC_LevelOne.PC_LevelOne_C"))
      (set `self.PlayerController` _returnvalue_7))
    (:`then_2`
      (`KismetArrayLibrary.Array_Set` (`.CamArray` (`self.CamArray`)) 0 (`.SpecCam_Free` (`self.SpecCam_Free`)))
      (`KismetArrayLibrary.Array_Set` (`.CamArray` (`self.CamArray`)) 1 (`.SpecCam_Front` (`self.SpecCam_Front`)))
      (`KismetArrayLibrary.Array_Set` (`.CamArray` (`self.CamArray`)) 2 (`.SpecCam_Top` (`self.SpecCam_Top`)))
      (`KismetArrayLibrary.Array_Set` (`.CamArray` (`self.CamArray`)) 3 (`.SpecCam_POV` (`self.SpecCam_POV`))))
    (:`then_3`
      (bind _returnvalue_8 (`GameplayStatics.GetActorOfClass` "/Game/VRMotionTracking/Blueprints/VRPawn_lvl1.VRPawn_lvl1_C"))
      (`self.K2_AttachToComponent` (`.SpecCam_POV` (`self.SpecCam_POV`)) (`/Game/VRMotionTracking/Blueprints/VRPawn_lvl1.HMDGimbal` _returnvalue_8) "None" "SnapToTarget" "SnapToTarget" "SnapToTarget" true))))

(event `/Camera/Select`
  (params (Message :type "OSCMessage Structure"))
  (bind _value (`OSCManager.GetInt32` Message))
  (switch `int` _value
    (:`0`
      (`self.DeactivateCams`
        (:`Out`
          (`HeadMountedDisplayFunctionLibrary.SetSpectatorScreenTexture` "/Engine/ArtTools/RenderToTexture/Textures/127grey.127grey"))))
    (:`1`
      (`self.SetCam` 1))
    (:`2`
      (`self.SetCam` 2))
    (:`3`
      (`self.SetCam` 3))
    (:`4`
      (`self.SetCam` 4))))

(event `Refresh Cam Pos`
  (bind _cam_current_vector (`self.cam current vector`))
  (bind _cam_target_vector (`self.cam target vector`))
  ;[0.481 0.5544 1] POS ROT Interpolation
  (set `self.cam current vector` (`SceneComponent.K2_GetComponentLocation` (`/Game/VRMotionTracking/Blueprints/OSCControl/bp_CAMERAS.DefaultSceneRoot` (`|GetArrayItem` (`.CamArray` (`self.CamArray`))))))
  (set `self.cam target vector` (`KismetMathLibrary.MakeVector` (`self.free cam x`) (`self.free cam y`) (`self.free cam z`)))
  (if (!= _cam_current_vector _cam_target_vector :`ErrorTolerance` 0.0001)
    (bind (_direction _alpha) (`Timeline|LI_Cam_Pos` :!via `PlayFromStart`)
      (:`Update`
        (`SceneComponent.K2_SetWorldLocation` (`/Game/VRMotionTracking/Blueprints/OSCControl/bp_CAMERAS.DefaultSceneRoot` (`|GetArrayItem` (`.CamArray` (`self.CamArray`)))) (`KismetMathLibrary.VLerp` _cam_current_vector _cam_target_vector _alpha) false false)))))

(event `StartInterp`
  (bind _li_cam_pos (`self.LI_Cam_Pos`))
  (bind _li_cam_rot (`self.LI_Cam Rot`))
  ;[0.481 0.5544 1] POS ROT Interpolation
  (`|ExecutionSequence`
    (:`then_0`
      (`TimelineComponent.SetPlayRate` _li_cam_pos (/ 1.0 (/ (`self.cam Pos Interpolation time in ms`) 1000.0)))
      (`TimelineComponent.Stop` _li_cam_pos)
      (`self.Refresh Cam Pos`))
    (:`then_1`
      (`TimelineComponent.SetPlayRate` _li_cam_rot (/ 1.0 (/ (`self.cam rot interpolation time in ms`) 1000.0)))
      (`TimelineComponent.Stop` _li_cam_rot)
      (`self.Refresh Cam Rot`))))

(event `/camera/locktoavatar`
  (params (Message :type "OSCMessage Structure"))
  (bind _value (`OSCManager.GetInt32` Message))
  (switch `int` _value
    (:`0`
      (for _array_element (`.CamArray` (`self.CamArray`))
        (if (!= _array_element null)
          (set `/Game/VRMotionTracking/Blueprints/OSCControl/bp_CAMERAS.LockCameraToAvatar` false _array_element)
          (bind _camdefaultrelativetransform (`/Game/VRMotionTracking/Blueprints/OSCControl/bp_CAMERAS.CamDefaultRelativeTransform` _array_element))
          (`SceneComponent.K2_SetRelativeRotation` (`/Game/VRMotionTracking/Blueprints/OSCControl/bp_CAMERAS.DefaultSceneRoot` _array_element) (`KismetMathLibrary.MakeRotator` 0.0 (.pitch (.rotation _camdefaultrelativetransform)) (.yaw (.rotation _camdefaultrelativetransform))) false false))))
    (:`1`
      (for _array_element_2 (`.CamArray` (`self.CamArray`))
        (if (!= _array_element_2 null)
          (set `/Game/VRMotionTracking/Blueprints/OSCControl/bp_CAMERAS.LockCameraToAvatar` true _array_element_2))))))

(event `Refresh Cam Rot`
  (bind _cam_current_rot (`self.cam current rot`))
  (bind _cam_target_rot (`self.cam target rot`))
  (bind _output (`|GetArrayItem` (`.CamArray` (`self.CamArray`))))
  ;[0.481 0.5544 1] POS ROT Interpolation
  (set `self.cam current rot` (`SceneComponent.K2_GetComponentRotation` (`/Game/VRMotionTracking/Blueprints/OSCControl/bp_CAMERAS.DefaultSceneRoot` (`|GetArrayItem` (`.CamArray` (`self.CamArray`))))))
  (set `self.cam target rot` (`KismetMathLibrary.MakeRotator` 0.0 (`self.free cam pitch`) (`self.free cam yaw`)))
  (if (!= _cam_current_rot _cam_target_rot :`ErrorTolerance` 0.0001)
    (if (`/Game/VRMotionTracking/Blueprints/OSCControl/bp_CAMERAS.CameraIsLockable` _output)
      (if (not (`/Game/VRMotionTracking/Blueprints/OSCControl/bp_CAMERAS.LockCameraToAvatar` _output))
        (bind (_direction _alpha) (`Timeline|LI_Cam Rot` :!via `PlayFromStart` :!label _label)
          (:`Update`
            (bind (_returnvalue_roll _returnvalue_pitch _returnvalue_yaw) (`KismetMathLibrary.BreakRotator` (`KismetMathLibrary.RLerp` _cam_current_rot _cam_target_rot _alpha true)))
            (`SceneComponent.K2_SetWorldRotation` (`/Game/VRMotionTracking/Blueprints/OSCControl/bp_CAMERAS.DefaultSceneRoot` (`|GetArrayItem` (`.CamArray` (`self.CamArray`)))) (`KismetMathLibrary.MakeRotator` 0.0 _returnvalue_pitch _returnvalue_yaw) false false))))
      (else
        (goto _label :!via `PlayFromStart`)))))

(event `/camera/zoom`
  (params (Message :type "OSCMessage Structure"))
  (bind _value (`OSCManager.GetFloat` Message))
  (set `self.field of view` (`KismetMathLibrary.MapRangeClamped` _value 0.0 1.0 120.0 20.0)))

(event `self.ReceiveTick`
  (params (DeltaSeconds :type "Float (single-precision)"))
  ;[1 1 1] FOV Interpolation
  (`|ExecutionSequence`
    (:`then_0`
      (for _array_element (`.CamArray` (`self.CamArray`))
        (`|ExecutionSequence`
          (:`then_0`
            (bind _camera (`/Game/VRMotionTracking/Blueprints/OSCControl/bp_CAMERAS.Camera` _array_element))
            (if (`ActorComponent.IsActive` _camera)
              (`CameraComponent.SetFieldOfView` _camera (`KismetMathLibrary.FInterpTo` (`CameraComponent.FieldOfView` _camera) (`self.field of view`) DeltaSeconds (`self.fov interp speed`)))))
          (:`then_1`
            (bind _scenecapturecomponent2d (`/Game/VRMotionTracking/Blueprints/OSCControl/bp_CAMERAS.SceneCaptureComponent2D` _array_element))
            (if (`ActorComponent.IsActive` _scenecapturecomponent2d)
              (set `SceneCaptureComponent2D.FOVAngle` (`KismetMathLibrary.FInterpTo` (`SceneCaptureComponent2D.FOVAngle` _scenecapturecomponent2d) (`self.field of view`) DeltaSeconds (`self.fov interp speed`)) _scenecapturecomponent2d))))))))

(event `/camera/free/pos/x`
  (params (Message :type "OSCMessage Structure"))
  (bind _value (`OSCManager.GetFloat` Message))
  (set `self.free cam x` (`KismetMathLibrary.Lerp` (`self.xmin`) (`self.xmax`) _value))
  (`self.StartInterp`))

(event `/camera/free/pos/y`
  (params (Message :type "OSCMessage Structure"))
  (bind _value (`OSCManager.GetFloat` Message))
  (set `self.free cam y` (`KismetMathLibrary.Lerp` (`self.ymin`) (`self.ymax`) _value))
  (`self.StartInterp`))

(event `/camera/free/pos/z`
  (params (Message :type "OSCMessage Structure"))
  (bind _value (`OSCManager.GetFloat` Message))
  (set `self.free cam z` (`KismetMathLibrary.Lerp` (`self.zmin`) (`self.zmax`) _value))
  (`self.StartInterp`))

(event `/camera/free/rot/pitch`
  (params (Message :type "OSCMessage Structure"))
  (bind _value (`OSCManager.GetFloat` Message))
  (if (`/Game/VRMotionTracking/Blueprints/OSCControl/bp_CAMERAS.LockCameraToAvatar` (`.SpecCam_Main` (`self.SpecCam_Main`)))
    (`KismetSystemLibrary.PrintString` "camera locked to avatar" true true (struct :`R` 1.0 :`B` 0.115187 :`A` 1.0))
    (elif (`KismetMathLibrary.InRange_FloatFloat` _value 0.0 0.25)
      (set `self.free cam pitch` (`KismetMathLibrary.MapRangeClamped` _value 0.0 0.25 0.0 89.9))
      (`self.StartInterp`)
      (elif (`KismetMathLibrary.InRange_FloatFloat` _value 0.75)
        (set `self.free cam pitch` (`KismetMathLibrary.MapRangeClamped` _value 0.75 1.0 -89.9))
        (`self.StartInterp`)))))

(event `/camera/free/rot/yaw`
  (params (Message :type "OSCMessage Structure"))
  (bind _value (`OSCManager.GetFloat` Message))
  (if (`/Game/VRMotionTracking/Blueprints/OSCControl/bp_CAMERAS.LockCameraToAvatar` (`.SpecCam_Main` (`self.SpecCam_Main`)))
    (`KismetSystemLibrary.PrintString` "camera locked to avatar" true true (struct :`R` 1.0 :`B` 0.115187 :`A` 1.0))
    (else
      (set `self.free cam yaw` (`KismetMathLibrary.MapRangeClamped` _value 0.0 1.0 0.1 359.9))
      (`self.StartInterp`))))

(fn `SetCam`
  (params (CamNumToActivate :type Integer))
  (bind _playercontroller (`self.PlayerController`))
  (`self.DeactivateCams`
    (:`Out`
      (if (`/Game/VRMotionTracking/Blueprints/VRPawn_lvl1.HMD Active` (`self.VRPawn_lvl1`))
        (switch `int` CamNumToActivate
          (:`1`
            (`self.Enable Capture` (`.SpecCam_Free` (`self.SpecCam_Free`)))
            (`HeadMountedDisplayFunctionLibrary.SetSpectatorScreenTexture` null)
            (`HeadMountedDisplayFunctionLibrary.SetSpectatorScreenMode` "Texture"))
          (:`2`
            (`self.Enable Capture` (`.SpecCam_Front` (`self.SpecCam_Front`)))
            (`HeadMountedDisplayFunctionLibrary.SetSpectatorScreenTexture` null)
            (`HeadMountedDisplayFunctionLibrary.SetSpectatorScreenMode` "Texture"))
          (:`3`
            (`self.Enable Capture` (`.SpecCam_Top` (`self.SpecCam_Top`)))
            (`HeadMountedDisplayFunctionLibrary.SetSpectatorScreenTexture` null)
            (`HeadMountedDisplayFunctionLibrary.SetSpectatorScreenMode` "Texture"))
          (:`4`
            (`self.Enable Capture` (`.SpecCam_POV` (`self.SpecCam_POV`)))
            (`HeadMountedDisplayFunctionLibrary.SetSpectatorScreenTexture` null)
            (`HeadMountedDisplayFunctionLibrary.SetSpectatorScreenMode` "Texture")))
        (else
          (switch `int` CamNumToActivate
            (:`1`
              (`/Game/VRMotionTracking/Blueprints/PC_LevelOne.SetCam1` _playercontroller))
            (:`2`
              (`/Game/VRMotionTracking/Blueprints/PC_LevelOne.SetCam2` _playercontroller))
            (:`3`
              (`/Game/VRMotionTracking/Blueprints/PC_LevelOne.SetCam3` _playercontroller))
            (:`4`
              (`/Game/VRMotionTracking/Blueprints/PC_LevelOne.SetCam4` _playercontroller))))))))

(fn `UserConstructionScript`)