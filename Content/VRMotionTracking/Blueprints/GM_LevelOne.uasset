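; GM_LevelOne is the game mode for level one of a VR motion tracking project, handling the handover of a player controller to the avatar.
; PossessPlayerToAvatar finds the level's VRPawn_lvl1, possesses it after a short delay, then teleports its root to the Bp_PlayerStart transform.
; BeginPlay and Tick are empty, and the spectator-screen HUD render-target logic in ShowSpecHUD is disconnected, so it never runs.
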(event `self.ReceiveBeginPlay`)

(event `PossessPlayerToAvatar`
  (params (Controller :type "Controller Object Reference"))
  (`/Engine/EditorBlueprintResources/StandardMacros.IsValid` Controller
    (:`Is Valid`
      (bind _returnvalue (`GameplayStatics.GetActorOfClass` "/Game/VRMotionTracking/Blueprints/VRPawn_lvl1.VRPawn_lvl1_C"))
      (`KismetSystemLibrary.Delay` 0.2)
      (`Controller.Possess` Controller _returnvalue)
      (bind _returnvalue_2 (`GameplayStatics.GetActorOfClass` "/Game/VRMotionTracking/Blueprints/bp_PlayerStart.bp_PlayerStart_C"))
      (`SceneComponent.K2_SetWorldTransform` (`/Game/VRMotionTracking/Blueprints/VRPawn_lvl1.DefaultSceneRoot` _returnvalue) (`self.GetTransform` _returnvalue_2) false true))))

(fn `ShowSpecHUD`)

(fn `UserConstructionScript`)