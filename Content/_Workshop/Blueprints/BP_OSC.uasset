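; BP_OSC lets external OSC messages control sun lighting and object scale in the level at runtime.
; On BeginPlay it starts a listening OSC server on port 8000 and finds the BP_LightControl actor.
; Received messages are routed by address path to change sun color or intensity, or uniformly scale ScaleObject, with debug prints.
; The separate R, G and B addresses share one color call fed by each branch's float output.
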(event `self.ReceiveBeginPlay`
  (bind _returnvalue (`OSCManager.CreateOSCServer` "" 8000 false true "" null))
  (bind _output_get (set `self.OSCServer` _returnvalue))
  (add `OSCServer.OnOscMessageReceived` _output_get (delegate `OSCMessageReceived`))
  (bind _returnvalue_2 (`GameplayStatics.GetActorOfClass` "/Game/_Workshop/Blueprints/BP_LightControl.BP_LightControl_C"))
  (set `self.BP_LightControl` _returnvalue_2))

(event `OSCMessageReceived`
  (params (Message :type "OSCMessage Structure (by ref)") (IPAddress :type String) (Port :type Integer))
  (bind _returnvalue (`OSCManager.GetOSCMessageAddress` Message))
  (bind _returnvalue_2 (`OSCManager.GetOSCAddressFullPath` _returnvalue))
  (`KismetSystemLibrary.PrintString` _returnvalue_2 true true (struct :`R` 1.0 :`G` 1.0 :`B` 1.0 :`A` 1.0) 20.0)
  (switch `string` _returnvalue_2
    (:`/light/sun/r`
      ;[1 0.9452 0.243] Sun Light
      (bind _value (`OSCManager.GetFloat` Message))
      (`KismetSystemLibrary.PrintString` (`KismetStringLibrary.Conv_DoubleToString` _value) true false (struct :`G` 1.0 :`A` 1.0) 20.0)
      (`/Game/_Workshop/Blueprints/BP_LightControl.ChangeSunLightColor` (`self.BP_LightControl`) (make `LinearColor` _value (stale _value_2) (stale _value_3) 1.0) :!label _label))
    (:`/light/sun/g`
      (bind _value_2 (`OSCManager.GetFloat` Message))
      (`KismetSystemLibrary.PrintString` (`KismetStringLibrary.Conv_DoubleToString` _value_2) true false (struct :`G` 1.0 :`A` 1.0) 20.0)
      (goto _label))
    (:`/light/sun/b`
      (bind _value_3 (`OSCManager.GetFloat` Message))
      (`KismetSystemLibrary.PrintString` (`KismetStringLibrary.Conv_DoubleToString` _value_3) true false (struct :`G` 1.0 :`A` 1.0) 20.0)
      (goto _label))
    (:`/light/sun/intensity`
      (bind _value_4 (`OSCManager.GetFloat` Message))
      (`KismetSystemLibrary.PrintString` (`KismetStringLibrary.Conv_DoubleToString` _value_4) true false (struct :`G` 1.0 :`A` 1.0) 20.0)
      (`/Game/_Workshop/Blueprints/BP_LightControl.ChangeSunLightIntensity` (`self.BP_LightControl`) _value_4))
    (:`/sphere/scale`
      ;[0.3833 1 0.8388] ScaleObject
      (bind _value_5 (`OSCManager.GetFloat` Message))
      (`KismetSystemLibrary.PrintString` (`KismetStringLibrary.Conv_DoubleToString` _value_5) true false (struct :`G` 1.0 :`A` 1.0) 20.0)
      (`self.SetActorScale3D` (`self.ScaleObject`) (`KismetMathLibrary.MakeVector` _value_5 _value_5 _value_5)))))

(fn `UserConstructionScript`)